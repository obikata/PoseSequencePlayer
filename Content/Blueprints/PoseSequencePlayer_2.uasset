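; Pose sequence player that replays recorded sensor-to-object poses from a data table, moving a SensorFrame relative to a tumbling ObjectFrame.
; PlayPoseSequence places both frames after a delay and sets READY.
; Tick spins the object and interpolates inverted, axis-flipped poses between adjacent rows at PlaySpeed.
; Each new row logs its pose and flashes a SpotLight with distance-scaled intensity, until a missing row flags DONE.
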(event `PlayPoseSequence`
  (bind _scale (`self.Scale`))
  (bind _objectframe (`self.ObjectFrame`))
  (bind _returnvalue (`KismetStringLibrary.Conv_IntToString` (`self.CurrentPoseID`)))
  ;[1 1 1] Initialize Pose
  (`KismetSystemLibrary.Delay` 3.0)
  (if (not (`self.READY`))
    (bind _returnvalue_2 (`|GetDataTableRow` "/Game/DataTables/UE5_DataTables_2.UE5_DataTables_2" (`KismetStringLibrary.Conv_StringToName` _returnvalue))
      (:`then`
        ;[1 1 1] Set Initial Object Pose relative to Sensor and Modify Orbital Plane
        (bind _returnvalue_3 (`|GetDataTableRow` "/Game/DataTables/UE5_DataTables_2.UE5_DataTables_2" "0")
          (:`then`
            (bind (_timestamp _x _y _z _qw _qx _qy _qz) (break `/Game/DataTables/PoseSequenceData` _returnvalue_3))
            (`SceneComponent.K2_SetRelativeLocationAndRotation` _objectframe (1500.0 0.0 0.0) (`KismetMathLibrary.Quat_Rotator` (`KismetMathLibrary.MakeQuat` (* _qx -1.0) _qy (* _qz -1.0) _qw)) false false)
            (`SceneComponent.K2_SetRelativeRotation` _objectframe (`KismetMathLibrary.Quat_Rotator` (`KismetMathLibrary.Quat_MakeFromEuler` (`KismetMathLibrary.MakeVector` 0.0 -90.0))) false false)
            (bind (_timestamp_2 _x_2 _y_2 _z_2 _qw_2 _qx_2 _qy_2 _qz_2) (break `/Game/DataTables/PoseSequenceData` _returnvalue_2))
            (bind _returnvalue_4 (`KismetMathLibrary.Quat_Inversed` (`KismetMathLibrary.MakeQuat` (* _qx_2 -1.0) _qy_2 (* _qz_2 -1.0) _qw_2)))
            (`SceneComponent.K2_SetRelativeLocationAndRotation` (`self.SensorFrame`) (`KismetMathLibrary.Quat_RotateVector` _returnvalue_4 (`KismetMathLibrary.NegateVector` (`KismetMathLibrary.MakeVector` (* _scale (+ (`self.OffsetX`) _x_2)) (* _scale (+ (`self.OffsetY`) (* _y_2 -1.0))) (* _scale (+ (`self.OffsetZ`) _z_2))))) (`KismetMathLibrary.Quat_Rotator` _returnvalue_4) false false)
            (`KismetSystemLibrary.PrintString` "#, X, Y, Z, Roll, Pitch, Yaw" true true (struct :`G` 0.66 :`B` 1.0 :`A` 1.0) 20.0)
            (`KismetSystemLibrary.PrintString` (`KismetStringLibrary.Concat_StrStr` _returnvalue ",   " (`self.GetFloatAsText` _x_2) ",   " (`self.GetFloatAsText` _y_2) ",   " (`self.GetFloatAsText` _z_2) ",   " (`KismetStringLibrary.Conv_IntToString` (`KismetMathLibrary.Round` (.roll (`KismetMathLibrary.Quat_Rotator` (`KismetMathLibrary.MakeQuat` _qx_2 _qy_2 _qz_2 _qw_2))))) ",   " (`KismetStringLibrary.Conv_IntToString` (`KismetMathLibrary.Round` (.pitch (`KismetMathLibrary.Quat_Rotator` (`KismetMathLibrary.MakeQuat` _qx_2 _qy_2 _qz_2 _qw_2))))) ",   " (`KismetStringLibrary.Conv_IntToString` (`KismetMathLibrary.Round` (.yaw (`KismetMathLibrary.Quat_Rotator` (`KismetMathLibrary.MakeQuat` _qx_2 _qy_2 _qz_2 _qw_2)))))) true true (struct :`G` 0.66 :`B` 1.0 :`A` 1.0) 20.0)
            (`KismetSystemLibrary.Delay` 3.0)
            (set `self.READY` true)
            (set `self.DONE` false)))))))

(event `self.ReceiveTick`
  (params (DeltaSeconds :type "Float (single-precision)"))
  (bind _ready (`self.READY`))
  (bind _scale (`self.Scale`))
  (bind _offsetx (`self.OffsetX`))
  (bind _offsety (`self.OffsetY`))
  (bind _scale_2 (`self.Scale`))
  (bind _spotlight (`self.SpotLight`))
  (bind _offsetz (`self.OffsetZ`))
  (bind _returnvalue (* (`self.PlaySpeed`) DeltaSeconds))
  (bind _returnvalue_2 (+ (* _returnvalue (`KismetMathLibrary.Conv_BoolToDouble` _ready)) (`self.ElapsedTime`)))
  (bind _returnvalue_3 (`KismetMathLibrary.FFloor` _returnvalue_2))
  (bind _returnvalue_4 (`KismetStringLibrary.Conv_IntToString` _returnvalue_3))
  (bind _returnvalue_5 (- _returnvalue_2 _returnvalue_3))
  ;[1 1 1] TumblingMotion
  (`SceneComponent.K2_AddLocalRotation` (`self.ObjectFrame`) (`KismetMathLibrary.MakeRotator` (* _returnvalue 1.0) (* _returnvalue 0.0) (* _returnvalue 0.0)) false false)
  ;[1 1 1] Update Pose
  (if _ready
    (bind _returnvalue_6 (`|GetDataTableRow` "/Game/DataTables/UE5_DataTables_2.UE5_DataTables_2" (`KismetStringLibrary.Conv_StringToName` _returnvalue_4))
      (:`then`
        (bind _returnvalue_7 (`|GetDataTableRow` "/Game/DataTables/UE5_DataTables_2.UE5_DataTables_2" (`KismetStringLibrary.Conv_StringToName` (`KismetStringLibrary.Conv_IntToString` (`KismetMathLibrary.FCeil` _returnvalue_2))))
          (:`then`
            (bind (_timestamp _x _y _z _qw _qx _qy _qz) (break `/Game/DataTables/PoseSequenceData` _returnvalue_6))
            (bind _returnvalue_8 (`KismetMathLibrary.Quat_Inversed` (`KismetMathLibrary.MakeQuat` (* _qx -1.0) _qy (* _qz -1.0) _qw)))
            (bind (_timestamp_2 _x_2 _y_2 _z_2 _qw_2 _qx_2 _qy_2 _qz_2) (break `/Game/DataTables/PoseSequenceData` _returnvalue_7))
            (bind _returnvalue_9 (`KismetMathLibrary.Quat_Inversed` (`KismetMathLibrary.MakeQuat` (* _qx_2 -1.0) _qy_2 (* _qz_2 -1.0) _qw_2)))
            (`SceneComponent.K2_SetRelativeLocationAndRotation` (`self.SensorFrame`) (`KismetMathLibrary.VLerp` (`KismetMathLibrary.Quat_RotateVector` _returnvalue_8 (`KismetMathLibrary.NegateVector` (`KismetMathLibrary.MakeVector` (* _scale (+ _offsetx _x)) (* _scale (+ _offsety (* _y -1.0))) (* _scale (+ _offsetz _z))))) (`KismetMathLibrary.Quat_RotateVector` _returnvalue_9 (`KismetMathLibrary.NegateVector` (`KismetMathLibrary.MakeVector` (* _scale_2 (+ _offsetx _x_2)) (* _scale_2 (+ _offsety (* _y_2 -1.0))) (* _scale_2 (+ _offsetz _z_2))))) _returnvalue_5) (`KismetMathLibrary.RLerp` (`KismetMathLibrary.Quat_Rotator` _returnvalue_8) (`KismetMathLibrary.Quat_Rotator` _returnvalue_9) _returnvalue_5 true) false false)
            (set `self.ElapsedTime` _returnvalue_2)
            (`/Engine/EditorBlueprintResources/StandardMacros.CompareInt` _returnvalue_3 (`self.CurrentPoseID`)
              (:`>`
                (`KismetSystemLibrary.PrintString` (`KismetStringLibrary.Concat_StrStr` _returnvalue_4 ",   " (`self.GetFloatAsText` _x_2) ",   " (`self.GetFloatAsText` _y_2) ",   " (`self.GetFloatAsText` _z_2) ",   " (`KismetStringLibrary.Conv_IntToString` (`KismetMathLibrary.Round` (.roll (`KismetMathLibrary.Quat_Rotator` (`KismetMathLibrary.MakeQuat` _qx_2 _qy_2 _qz_2 _qw_2))))) ",   " (`KismetStringLibrary.Conv_IntToString` (`KismetMathLibrary.Round` (.pitch (`KismetMathLibrary.Quat_Rotator` (`KismetMathLibrary.MakeQuat` _qx_2 _qy_2 _qz_2 _qw_2))))) ",   " (`KismetStringLibrary.Conv_IntToString` (`KismetMathLibrary.Round` (.yaw (`KismetMathLibrary.Quat_Rotator` (`KismetMathLibrary.MakeQuat` _qx_2 _qy_2 _qz_2 _qw_2)))))) true true (struct :`G` 0.66 :`B` 1.0 :`A` 1.0) 20.0)
                (set `self.CurrentPoseID` _returnvalue_3)
                (if (not (stale _output_get))
                  (`SceneComponent.SetVisibility` _spotlight true false)
                  (bind _returnvalue_10 (+ (* (`self.A`) _x_2) (`self.B`)))
                  (`LightComponent.SetIntensity` _spotlight (* _returnvalue_10 _returnvalue_10))
                  (bind _output_get (set `self.LED` true))
                  (`KismetSystemLibrary.Delay` 0.25)
                  (`SceneComponent.SetVisibility` _spotlight false false)
                  (`KismetSystemLibrary.Delay` 0.75)
                  (set `self.LED` false)))))
          (:`RowNotFound`
            (bind _output_get_2 (set `self.DONE` true))
            (set `self.ElapsedTime` 0.0)
            (set `self.CurrentPoseID` 0)
            (set `self.READY` false)
            (`KismetSystemLibrary.PrintString` "DONE!" true true (struct :`G` 0.66 :`B` 1.0 :`A` 1.0) 20.0)
            (if _output_get_2
              (`SceneComponent.SetVisibility` _spotlight false false))))))))

(fn `GetDone`
  (returns (`Return Value` :type Boolean))
  (return (`self.DONE`)))

(fn `GetReady`
  (returns (`Return Value` :type Boolean))
  (return (`self.READY`)))

(fn `UserConstructionScript`)